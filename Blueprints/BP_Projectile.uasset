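; Projectile actor that flies along world X and destroys potions, enemies or itself on contact.
; Each tick it moves by its own ProjectileSpeed plus the player's current forward speed, so its motion stays relative to the moving player.
; Sphere overlap destroys a hit BP_Potion or BP_Enemy along with the projectile.
; Overlapping any static mesh component destroys only the projectile, checked before the enemy cast.
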(event OnComponentBeginOverlap(Sphere)
  (params (OverlappedComponent :type Primitive%20Component%20Object%20Reference) (OtherActor :type Actor%20Object%20Reference) (OtherComp :type Primitive%20Component%20Object%20Reference) (OtherBodyIndex :type Integer) (bFromSweep :type Boolean) (SweepResult :type Hit%20Result%20Structure%20%28by%20ref%29))
  (bind _asbp_potion (Utilities|Casting|CastToBP_Potion OtherActor)
    (:then
      (Actor|DestroyActor _asbp_potion)
      (Actor|DestroyActor))
    (:CastFailed
      (Utilities|Casting|CastToStaticMeshComponent OtherComp
        (:then
          (Actor|DestroyActor))
        (:CastFailed
          (bind _asbp_enemy (Utilities|Casting|CastToBP_Enemy OtherActor))
          (Actor|DestroyActor _asbp_enemy)
          (Actor|DestroyActor)
          (Development|PrintString "ENEMY HIT"))))))

(event EventBeginPlay)

(event Collision|EventActorBeginOverlap
  (params (OtherActor :type Actor%20Object%20Reference)))

(event EventTick
  (params (DeltaSeconds :type Float%20%28single-precision%29))
  (bind _asbp_player (Utilities|Casting|CastToBP_Player (Game|Player|GetPlayerPawn 0)))
  (Transformation|AddActorWorldOffset (Math|Vector|MakeVector (* DeltaSeconds (+ (Variables|/Game/InfiniteMatrix/Blueprints/BP_Player.BP_Player_C|GetForwardSpeedCurrent _asbp_player) (Variables|Default|GetProjectileSpeed))) 0.0 0.0)))

(fn ConstructionScript)